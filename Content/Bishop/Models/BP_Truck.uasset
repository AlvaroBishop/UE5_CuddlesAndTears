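; BP_Truck is a truck actor that periodically drives along the X axis to drop off groups of AI baby pawns.
; Tick accumulates a timer, playing a Timeline that sets the truck's X position once SpawnRate is exceeded, and reversing it otherwise.
; When X exactly equals a hard-coded endpoint, it resets the timer and SpawnBaby spawns NumberOfBabies BP_TopDownBaby pawns at random offsets from the truck.
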(event `self.ReceiveBeginPlay`
  (set `self.ActorStartLocation` (`self.K2_GetActorLocation`)))

(event `self.ReceiveTick`
  (params (DeltaSeconds :type "Float (single-precision)"))
  (bind (_returnvalue_x _returnvalue_y _returnvalue_z) (`KismetMathLibrary.BreakVector` (`self.K2_GetActorLocation`)))
  (set `self.SpawnTime` (+ DeltaSeconds (`self.SpawnTime`)))
  (if (> (`self.SpawnTime`) (`self.SpawnRate`))
    (bind (_direction _move) (`Timeline|Timeline` :!label _label)
      (:`Update`
        (`self.K2_SetActorLocation` (`KismetMathLibrary.MakeVector` _move _returnvalue_y _returnvalue_z))
        (if (== _returnvalue_x 700.0)
          (set `self.SpawnTime` 0.0)
          (`self.SpawnBaby`))))
    (else
      (goto _label :!via `Reverse`))))

(fn `SpawnBaby`
  (for _ (range 1 (+ (`self.NumberOfBabies`) 1))
    (`AIBlueprintHelperLibrary.SpawnAIFromClass` "/Game/Paul/BluePrints/BP_TopDownBaby.BP_TopDownBaby_C" null (+ (`self.K2_GetActorLocation`) (`KismetMathLibrary.MakeVector` (`KismetMathLibrary.RandomFloatInRange` -300.0 -400.0) (`KismetMathLibrary.RandomFloatInRange` 0.0 60.0))) (struct) true null)))

(fn `UserConstructionScript`)