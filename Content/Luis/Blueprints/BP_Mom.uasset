(event `self.ReceiveTick`
  (params (DeltaSeconds :type "Float (single-precision)"))
  (`KismetSystemLibrary.Delay` 15.0)
  (if (not (`self.CanTurnIn`))
    (set `self.CanTurnIn` true)
    (`GameplayStatics.PlaySound2D` "/Game/Paul/Sounds/Mom.Mom" 1.0 1.0 0.0 null null)
    (`SceneComponent.SetHiddenInGame` (`self.Mom Text`) false false)
    (`SceneComponent.SetHiddenInGame` (`self.PaperSprite`) false false)))

(event `self.Sphere.OnComponentBeginOverlap`
  (params (OverlappedComponent :type "PrimitiveComponent Object Reference") (OtherActor :type "Actor Object Reference") (OtherComp :type "PrimitiveComponent Object Reference") (OtherBodyIndex :type Integer) (bFromSweep :type Boolean) (SweepResult :type "HitResult Structure (by ref)"))
  (bind _asbp_top_down_char (cast `/Game/Bishop/Character/BP_TopDownChar` OtherActor))
  (if (`self.CanTurnIn`)
    (if (`/Game/Bishop/Character/BP_TopDownChar.HasBaby` _asbp_top_down_char)
      (set `/Game/Bishop/Character/BP_TopDownChar.Money` (+ (`/Game/Bishop/Character/BP_TopDownChar.Money` _asbp_top_down_char) 100) _asbp_top_down_char)
      (set `/Game/Bishop/Character/BP_TopDownChar.HasBaby` false _asbp_top_down_char)
      (`SceneComponent.SetHiddenInGame` (`/Game/Bishop/Character/BP_TopDownChar.PaperSprite` _asbp_top_down_char) true false)
      (set `self.CanTurnIn` false)
      (`SceneComponent.SetHiddenInGame` (`self.Mom Text`) true false)
      (`GameplayStatics.PlaySound2D` "/Game/Paul/Sounds/ThankYou.ThankYou" 1.0 1.0 0.0 null null)
      (`SceneComponent.SetHiddenInGame` (`self.PaperSprite`) true false))))

(fn `UserConstructionScript`)